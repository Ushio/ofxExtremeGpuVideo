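; BP_GpuVideoPlayer is an actor that plays a GPU video file on its PlayerPlane mesh.
; On BeginPlay it puts a dynamic instance of VideoRenderMaterial on the plane and loads the GV video from a path relative to the project Content directory.
; Each Tick it accumulates playback time, wraps it by video length when looping, and feeds the rendered texture into the material's GpuVideoTexture parameter.
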(event EventBeginPlay
  ;[1 1 1] Create Material Instance
  (bind _returnvalue (Rendering|Material|CreateDynamicMaterialInstance "/Game/VideoRenderMaterial.VideoRenderMaterial" "None" "None" :!class /Script/Engine.KismetMaterialLibrary))
  (Rendering|Material|SetMaterial (Variables|Default|GetPlayerPlane) 0 _returnvalue)
  (bind _returnvalue_2 (Class|GpuVideoFunction|LoadGV (Class|BlueprintPathsLibrary|Combine (Utilities|Array|MakeArray (Class|BlueprintPathsLibrary|ConvertRelativePathtoFull (Class|BlueprintPathsLibrary|ProjectContentDir)) (Variables|Default|GetVideoFilePath))))))

(event Collision|EventActorBeginOverlap
  (params (OtherActor :type Actor%20Object%20Reference)))

(event EventTick
  (params (DeltaSeconds :type Float%20%28single-precision%29))
  (bind _output_get (Variables|Default|SetTotalTime (+ DeltaSeconds (Variables|Default|GetTotalTime))))
  (if (Variables|Default|GetIsLooping)
    (bind _returnvalue (Class|GpuVideoFunction|GetGpuVideoLength (stale EventBeginPlay _returnvalue_2)))
    (Variables|Default|SetTotalTime (Math|Float|%(Float) _output_get _returnvalue)))
  (bind _returnvalue_2 (Class|GpuVideoFunction|RenderGpuVideotoTexture (Variables|Default|GetTotalTime) (stale EventBeginPlay _returnvalue_2)))
  (Rendering|Material|SetTextureParameterValue (stale EventBeginPlay _returnvalue) "GpuVideoTexture" _returnvalue_2))

(fn ConstructionScript)